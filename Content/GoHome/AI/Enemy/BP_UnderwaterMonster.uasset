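; Underwater monster enemy that patrols between BP_AIPosition points of its patrol group, with all AI logic running on the server.
; Tick switches between moving, driven by an UnderwaterSteeringMovement component tracing from EyePoint, and waiting a random per-point time before picking another random point.
; A movement timeout and a distance-based stuck check force a new point.
; BeginPlay schedules a looping CheckForPlayer timer, but that function is absent here.
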(event `self.ReceiveBeginPlay`
  (`UnderwaterSteeringMovement.SetTraceStartComponent` (`self.UnderwaterSteeringMovement`) (`self.EyePoint`))
  (`/Engine/EditorBlueprintResources/ActorMacros.Switch Has Authority`
    (:`Authority`
      (bind _outactors (`GameplayStatics.GetAllActorsOfClass` "/Game/GoHome/AI/Enemy/BP_AIPosition.BP_AIPosition_C"))
      (set `self.AllPositions` _outactors)
      (`KismetSystemLibrary.K2_SetTimer` self "CheckForPlayer" 0.2 true)
      (`self.PickNextPatrolPosition`))))

(event `self.ReceiveTick`
  (params (DeltaSeconds :type "Float (single-precision)"))
  (`/Engine/EditorBlueprintResources/ActorMacros.Switch Has Authority`
    (:`Authority`
      (if (`self.IsRePosition`)
        (set `self.StuckTime` (+ (`self.StuckTime`) DeltaSeconds))
        (set `self.LastLocation` (`self.K2_GetActorLocation`))
        (if (> (`self.StuckTime`) (`self.StuckLimitTime`))
          (set `self.StuckTime` 0.0)
          (`self.PickNextPatrolPosition`)
          (else
            (switch `/Game/GoHome/AI/Enemy/E_MonsterState` (`self.State`) :!label _label
              (:`NewEnumerator0`
                (`self.PatrolMove`))
              (:`NewEnumerator1`
                (`self.PatrolWait`)))))
        (else
          (set `self.StuckTime` 0.0)
          (goto _label))))))

(fn `IsRePosition`
  (returns (ReturnValue :type Boolean))
  (return (< (`KismetMathLibrary.Vector_Distance` (`self.K2_GetActorLocation`) (`self.LastLocation`)) (`self.StuckCheckDistacne`))))

(fn `OnMoveTimeout`
  (`/Engine/EditorBlueprintResources/ActorMacros.Switch Has Authority`
    (:`Authority`
      (if (`self.bMoveTimeoutActive`)
        (set `self.bMoveTimeoutActive` false)
        (`self.PickNextPatrolPosition`)))))

(fn `PatrolMove`
  (bind _returnvalue (`self.K2_GetActorLocation` (`self.CurrentPosition`)))
  (`/Engine/EditorBlueprintResources/ActorMacros.Switch Has Authority`
    (:`Authority`
      (`/Engine/EditorBlueprintResources/StandardMacros.IsValid` (`self.CurrentPosition`)
        (:`Is Valid`
          (if (`UnderwaterSteeringMovement.Steering_HasArrived` (`self.UnderwaterSteeringMovement`) _returnvalue)
            (`UnderwaterSteeringMovement.Steering_Stop` (`self.UnderwaterSteeringMovement`))
            (set `self.bWaitTimerStarted` false)
            (set `self.State` "NewEnumerator1")
            (else
              (`UnderwaterSteeringMovement.Steering_MoveToLocation` (`self.UnderwaterSteeringMovement`) _returnvalue (`self.PatrolSpeed`) (`GameplayStatics.GetWorldDeltaSeconds`)))))
        (:`Is Not Valid`
          (`self.PickNextPatrolPosition`))))))

(fn `PatrolWait`
  (bind _currentposition (`self.CurrentPosition`))
  (`/Engine/EditorBlueprintResources/ActorMacros.Switch Has Authority`
    (:`Authority`
      (`UnderwaterSteeringMovement.Steering_Stop` (`self.UnderwaterSteeringMovement`))
      (if (`self.bWaitTimerStarted`)
        (return)
        (else
          (set `self.bWaitTimerStarted` true)
          (`KismetSystemLibrary.K2_SetTimer` self "PickNextPatrolPosition" (`KismetMathLibrary.RandomFloatInRange` (`/Game/GoHome/AI/Enemy/BP_AIPosition.WaitMin` _currentposition) (`/Game/GoHome/AI/Enemy/BP_AIPosition.WaitMax` _currentposition))))))))

(fn `PickNextPatrolPosition`
  (locals (Candidates :type "Array of /Game/GoHome/AI/Enemy/BP_AIPosition Object Reference") (index :type Integer) (Position :type "/Game/GoHome/AI/Enemy/BP_AIPosition Object Reference"))
  (bind _returnvalue (`KismetArrayLibrary.Array_Length` (`local.Candidates`)))
  (bind _returnvalue_2 (`KismetArrayLibrary.Array_Length` (`local.Candidates`)))
  (`/Engine/EditorBlueprintResources/ActorMacros.Switch Has Authority`
    (:`Authority`
      (`KismetArrayLibrary.Array_Clear` (`local.Candidates`))
      (for _array_element (`self.AllPositions`)
        (set `self.Array Element` _array_element)
        (`/Engine/EditorBlueprintResources/StandardMacros.IsValid` _array_element
          (:`Is Valid`
            (if (== (`/Game/GoHome/AI/Enemy/BP_AIPosition.GroupID` (`self.Array Element`)) (`self.PatrolGroupID`))
              (if (!= (`self.Array Element`) (`self.CurrentPosition`))
                (`KismetArrayLibrary.Array_Add` (`local.Candidates`) (`self.Array Element`)))))))
      (if (> _returnvalue 0)
        (set `local.index` (`KismetMathLibrary.RandomIntegerInRange` 0 (- _returnvalue 1)))
        (set `self.LastPosition` (`self.CurrentPosition`))
        (set `self.CurrentPosition` (`|GetArrayItem` (`local.Candidates`) (`local.index`)))
        (set `self.State` "NewEnumerator0")
        (`KismetSystemLibrary.K2_ClearTimer` self "OnMoveTimeout")
        (set `self.bMoveTimeoutActive` true)
        (`KismetSystemLibrary.K2_SetTimer` self "OnMoveTimeout" (`self.MoveTimeout`))
        (else
          (`KismetArrayLibrary.Array_Clear` (`local.Candidates`))
          (for _array_element_2 (`self.AllPositions`)
            (`/Engine/EditorBlueprintResources/StandardMacros.IsValid` _array_element_2
              (:`Is Valid`
                (if (== (`/Game/GoHome/AI/Enemy/BP_AIPosition.GroupID` (`self.Array Element`)) (`self.PatrolGroupID`))
                  (`KismetArrayLibrary.Array_Add` (`local.Candidates`) (`self.Array Element`))))))
          (if (> _returnvalue_2 0)
            (set `local.index` (`KismetMathLibrary.RandomIntegerInRange` 0 (- _returnvalue_2 1)))
            (set `self.LastPosition` (`self.CurrentPosition`))
            (set `self.CurrentPosition` (`|GetArrayItem` (`local.Candidates`) (`local.index`)))
            (set `self.State` "NewEnumerator0")
            (`KismetSystemLibrary.K2_ClearTimer` null "OnMoveTimeout")
            (set `self.bMoveTimeoutActive` true)
            (`KismetSystemLibrary.K2_SetTimer` null "OnMoveTimeout" (`self.MoveTimeout`))
            (else
              (set `self.State` "NewEnumerator1"))))))))

(fn `UserConstructionScript`)